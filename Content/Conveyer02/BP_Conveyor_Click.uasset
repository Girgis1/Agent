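; Conveyor actor that builds itself at BeginPlay between the player character's PosA and PosB, with debug spheres.
; A four-point spline, its inner points offset along endpoint facings, gets BP_SplineHandle actors plus spline-mesh belt, collision and rails.
; A looping timer pushes actors overlapping the collision meshes along the spline, sweeping Characters and reorienting others.
; Grabbed handles move their spline points, but the mesh refresh never reapplies segment endpoints.
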(event `self.ReceiveBeginPlay`
  (bind _spline (`self.Spline`))
  (bind _spline_2 (`self.Spline`))
  (bind _spline_3 (`self.Spline`))
  (bind _spline_4 (`self.Spline`))
  (bind _spline_5 (`self.Spline`))
  (bind _asbp_third_person_character (cast `/Game/ThirdPerson/Blueprints/BP_ThirdPersonCharacter` (`GameplayStatics.GetPlayerCharacter` 0)))
  (bind (_posa_location _posa_rotation) (`KismetMathLibrary.BreakTransform` (`/Game/ThirdPerson/Blueprints/BP_ThirdPersonCharacter.PosA` _asbp_third_person_character)))
  (set `self.0` _posa_location)
  (bind (_posb_location _posb_rotation) (`KismetMathLibrary.BreakTransform` (`/Game/ThirdPerson/Blueprints/BP_ThirdPersonCharacter.PosB` _asbp_third_person_character)))
  (bind _returnvalue (+ (* (`KismetMathLibrary.Vector_Distance` _posa_location _posb_location) (`self.SplineOffset`)) (`self.SplineOffset Padding`)))
  (set `self.1` (+ _posa_location (* (`KismetMathLibrary.GetForwardVector` _posa_rotation) _returnvalue)))
  (set `self.2` (+ _posb_location (* (`KismetMathLibrary.GetForwardVector` _posb_rotation) (* _returnvalue -1.0))))
  (set `self.3` _posb_location)
  (`KismetSystemLibrary.DrawDebugSphere` (`self.0`) 5.0 12 (struct :`R` 1.0 :`G` 1.0 :`B` 1.0 :`A` 1.0) 10.0)
  (`KismetSystemLibrary.DrawDebugSphere` (`self.1`) 5.0 12 (struct :`A` 1.0) 10.0)
  (`KismetSystemLibrary.DrawDebugSphere` (`self.2`) 5.0 12 (struct :`A` 1.0) 10.0)
  (`KismetSystemLibrary.DrawDebugSphere` (`self.3`) 5.0 12 (struct :`R` 1.0 :`G` 1.0 :`B` 1.0 :`A` 1.0) 10.0)
  (`SplineComponent.SetLocationAtSplinePoint` _spline 0 (`self.0`) "World" false)
  (`SplineComponent.SetSplinePointType` _spline 0 "Linear" false)
  (`SplineComponent.AddSplinePointAtIndex` _spline_3 (`self.1`) 1 "World" false)
  (`SplineComponent.SetSplinePointType` _spline_3 1 "Curve" false)
  (`SplineComponent.AddSplinePointAtIndex` _spline_2 (`self.2`) 2 "World" false)
  (`SplineComponent.SetSplinePointType` _spline_2 2 "Linear" false)
  (`SplineComponent.AddSplinePointAtIndex` (`self.Spline`) (`self.3`) 3 "World" true)
  (`KismetSystemLibrary.Delay` 1.0)
  (`SplineComponent.SetTangentAtSplinePoint` _spline_4 1 (* (`.Tangent` (`SplineComponent.GetLocationAndTangentAtSplinePoint` _spline_5 1 "World")) 5.0) "World" true)
  (`SplineComponent.SetTangentAtSplinePoint` _spline_4 2 (* (`.Tangent` (`SplineComponent.GetLocationAndTangentAtSplinePoint` _spline_5 2 "World")) 5.0) "World" true)
  (`KismetSystemLibrary.Delay` 1.0)
  (bind _returnvalue_2 (`|SpawnActorFromClass` "/Game/Conveyer02/BP_SplineHandle.BP_SplineHandle_C" (`KismetMathLibrary.MakeTransform` (`self.0`)) "Undefined" "MultiplyWithRoot" null null))
  (set `self.Handle0` _returnvalue_2)
  (bind _returnvalue_3 (`|SpawnActorFromClass` "/Game/Conveyer02/BP_SplineHandle.BP_SplineHandle_C" (`KismetMathLibrary.MakeTransform` (`self.1`)) "Undefined" "MultiplyWithRoot" null null))
  (set `self.Handle_1` _returnvalue_3)
  (bind _returnvalue_4 (`|SpawnActorFromClass` "/Game/Conveyer02/BP_SplineHandle.BP_SplineHandle_C" (`KismetMathLibrary.MakeTransform` (`self.2`)) "Undefined" "MultiplyWithRoot" null null))
  (set `self.Handle2` _returnvalue_4)
  (bind _returnvalue_5 (`|SpawnActorFromClass` "/Game/Conveyer02/BP_SplineHandle.BP_SplineHandle_C" (`KismetMathLibrary.MakeTransform` (`self.3`)) "Undefined" "MultiplyWithRoot" null null))
  (set `self.Handle3` _returnvalue_5)
  (`self.UpdateMesh` true))

(event `HandleGrabbed`
  (params (Grabbed :type Boolean))
  (bind _handle_1 (`self.Handle_1`))
  (bind _handle2 (`self.Handle2`))
  (bind _handle3 (`self.Handle3`))
  (bind _handle0 (`self.Handle0`))
  (if Grabbed
    (bind _asbp_third_person_character (cast `/Game/ThirdPerson/Blueprints/BP_ThirdPersonCharacter` (`GameplayStatics.GetPlayerCharacter` 0)))
    (`|ExecutionSequence`
      (:`then_0`
        (bind _hit_actor (`/Game/ThirdPerson/Blueprints/BP_ThirdPersonCharacter.Hit Actor` _asbp_third_person_character))
        (if (== _hit_actor _handle0)
          (`SplineComponent.SetLocationAtSplinePoint` (`self.Spline`) 0 (`SceneComponent.GetSocketLocation` (`/Game/Conveyer02/BP_SplineHandle.Handle` _handle0) "None") "World" true)
          (`KismetSystemLibrary.Delay` 1.0)
          (`KismetSystemLibrary.Delay` 0.1 :!label _label)
          (`KismetSystemLibrary.PrintString` "SPLINE GRAB UPDATED" true true (struct :`G` 0.66 :`B` 1.0 :`A` 1.0) 5.0)
          (`KismetSystemLibrary.Delay` 0.5)
          (`SplineMeshComponent.UpdateMesh` (`self.MeshComponents`))
          (`SplineMeshComponent.UpdateMesh` (`self.OverlappedComponents`))
          (`SplineMeshComponent.UpdateMesh` (`self.Rails`))))
      (:`then_1`
        (if (== _hit_actor _handle_1)
          (`SplineComponent.SetLocationAtSplinePoint` (`self.Spline`) 1 (`SceneComponent.GetSocketLocation` (`/Game/Conveyer02/BP_SplineHandle.Handle` _handle_1) "None") "World" true)
          (`KismetSystemLibrary.Delay` 1.0)
          (goto _label)))
      (:`then_2`
        (if (== _hit_actor _handle2)
          (`SplineComponent.SetLocationAtSplinePoint` (`self.Spline`) 2 (`SceneComponent.GetSocketLocation` (`/Game/Conveyer02/BP_SplineHandle.Handle` _handle2) "None") "World" true)
          (`KismetSystemLibrary.Delay` 1.0)
          (goto _label)))
      (:`then_3`
        (if (== _hit_actor _handle3)
          (`SplineComponent.SetLocationAtSplinePoint` (`self.Spline`) 3 (`SceneComponent.GetSocketLocation` (`/Game/Conveyer02/BP_SplineHandle.Handle` _handle3) "None") "World" true)
          (`KismetSystemLibrary.Delay` 1.0)
          (goto _label))))))

(event `UpdateMesh`
  (params (UpdateMesh :type Boolean))
  (bind _spline (`self.Spline`))
  (bind _spline_2 (`self.Spline`))
  (if UpdateMesh
    (for _index (range (+ (- (`SplineComponent.GetNumberOfSplinePoints` (`self.Spline`)) 2) 1))
      ;[1 1 1] Belt
      (bind _returnvalue (`AddComponent|NODE_AddSplineMeshComponent-26` :`bManualAttachment` true)) ; Belt
      (`KismetArrayLibrary.Array_Add` (`self.MeshComponents`) _returnvalue)
      (bind (_location _tangent) (`SplineComponent.GetLocationAndTangentAtSplinePoint` _spline _index "World"))
      (bind _returnvalue_2 (+ _index 1))
      (bind (_location_2 _tangent_2) (`SplineComponent.GetLocationAndTangentAtSplinePoint` _spline _returnvalue_2 "World"))
      (`SplineMeshComponent.SetStartAndEnd` _returnvalue _location _tangent _location_2 _tangent_2 true)
      (`MeshComponent.SetScalarParameterValueOnMaterials` _returnvalue "XScale" (/ (- (`SplineComponent.GetDistanceAlongSplineAtSplinePoint` _spline_2 _returnvalue_2) (`SplineComponent.GetDistanceAlongSplineAtSplinePoint` _spline_2 _index)) 20.0))
      ;[1 1 1] Collision Mesh
      (bind _returnvalue_3 (`AddComponent|NODE_AddSplineMeshComponent-28` :`bManualAttachment` true)) ; Collision Box
      (`KismetArrayLibrary.Array_Add` (`self.OverlappedComponents`) _returnvalue_3)
      (`SplineMeshComponent.SetStartAndEnd` _returnvalue_3 _location _tangent _location_2 _tangent_2 true)
      ;[1 1 1] Rails
      (bind _returnvalue_4 (`AddComponent|NODE_AddSplineMeshComponent-27` :`bManualAttachment` true)) ; Rails
      (`KismetArrayLibrary.Array_Add` (`self.Rails`) _returnvalue_4)
      (`SplineMeshComponent.SetStartAndEnd` _returnvalue_4 _location _tangent _location_2 _tangent_2 true)
      (`self.UpdateMesh` false)
      (`self.Conveyor On`))))

(event `Conveyor On`
  ;[0 0 0] This is my core one i'm trying to intergrate into the others
  (`KismetSystemLibrary.K2_SetTimerDelegate` (delegate `MoveObjects`) 0.01 true))

(event `MoveObjects`
  (bind _returnvalue (`SceneComponent.K2_GetComponentRotation` (`self.DefaultSceneRoot`)))
  ;[0 0 0] This is my core one i'm trying to intergrate into the others
  (set `self.MovedActors` (`|MakeArray` self :!type "Actor Object Reference"))
  (for _array_element (`self.OverlappedComponents`)
    (for _array_element_2 (`PrimitiveComponent.GetOverlappingActors` _array_element null)
      (if (== (`KismetArrayLibrary.Array_Find` (`self.MovedActors`) _array_element_2) -1)
        (cast `Character` _array_element_2
          (:`then`
            (bind _returnvalue_2 (`KismetMathLibrary.GreaterGreater_VectorRotator` (* (`SplineComponent.FindDirectionClosestToWorldLocation` (`self.Spline`) (`self.K2_GetActorLocation` _array_element_2) "Local") (`self.DynamicSpeed`)) _returnvalue))
            (`self.K2_AddActorWorldOffset` _array_element_2 _returnvalue_2 true false))
          (:`CastFailed`
            (`self.K2_AddActorWorldOffset` _array_element_2 _returnvalue_2 false false)
            (`/Engine/EditorBlueprintResources/StandardMacros.IsValid` _array_element_2
              (:`Is Valid`
                (bind _returnvalue_3 (`self.K2_GetActorLocation` _array_element_2))
                (bind (_returnvalue_roll _returnvalue_pitch) (`KismetMathLibrary.BreakRotator` (* (`SplineComponent.FindRotationClosestToWorldLocation` (`self.Spline`) _returnvalue_3 "Local") -1.0)))
                (`self.K2_SetActorRotation` _array_element_2 (`KismetMathLibrary.ComposeRotators` (`KismetMathLibrary.MakeRotator` 0.0 0.0 (`KismetAnimationLibrary.CalculateDirection` (`SplineComponent.FindTangentClosestToWorldLocation` (`self.Spline`) _returnvalue_3 "Local") _returnvalue)) (`KismetMathLibrary.MakeRotator` _returnvalue_roll _returnvalue_pitch)) false))
              (:`Is Not Valid`
                _))))
        (`KismetArrayLibrary.Array_Add` (`self.MovedActors`) _array_element_2)))))

(fn `UserConstructionScript`)