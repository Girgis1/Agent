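; Hologram variant of a spline conveyor, apparently work in progress, built to push overlapping actors along its path.
; ConveyorOn loops a 0.01-second timer on MoveObjects, moving each overlapped actor once along the nearest spline direction, sweeping Characters and rotating others to the curve.
; Spline placement from player points, belt/collision/rail mesh generation and belt material animation are all disconnected.
; Thus nothing here calls ConveyorOn or fills its overlap list.
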(event `self.ReceiveBeginPlay`
  ;[0.02969 0.2656 0] Comment
)

(event `self.ReceiveTick`
  (params (DeltaSeconds :type "Float (single-precision)")))

(event `Conveyor On`
  ;[0 0 0] This is my core one i'm trying to intergrate into the others
  (`KismetSystemLibrary.K2_SetTimerDelegate` (delegate `MoveObjects`) 0.01 true))

(event `MoveObjects`
  (bind _returnvalue (`SceneComponent.K2_GetComponentRotation` (`self.DefaultSceneRoot`)))
  ;[0 0 0] This is my core one i'm trying to intergrate into the others
  (set `self.MovedActors` (`|MakeArray` self :!type "Actor Object Reference"))
  (for _array_element (`self.OverlappedComponents`)
    (for _array_element_2 (`PrimitiveComponent.GetOverlappingActors` _array_element null)
      (if (== (`KismetArrayLibrary.Array_Find` (`self.MovedActors`) _array_element_2) -1)
        (cast `Character` _array_element_2
          (:`then`
            (bind _returnvalue_2 (`KismetMathLibrary.GreaterGreater_VectorRotator` (* (`SplineComponent.FindDirectionClosestToWorldLocation` (`self.Spline`) (`self.K2_GetActorLocation` _array_element_2) "Local") (`self.DynamicSpeed`)) _returnvalue))
            (`self.K2_AddActorWorldOffset` _array_element_2 _returnvalue_2 true false))
          (:`CastFailed`
            (`self.K2_AddActorWorldOffset` _array_element_2 _returnvalue_2 false false)
            (`/Engine/EditorBlueprintResources/StandardMacros.IsValid` _array_element_2
              (:`Is Valid`
                (bind _returnvalue_3 (`self.K2_GetActorLocation` _array_element_2))
                (bind (_returnvalue_roll _returnvalue_pitch) (`KismetMathLibrary.BreakRotator` (* (`SplineComponent.FindRotationClosestToWorldLocation` (`self.Spline`) _returnvalue_3 "Local") -1.0)))
                (`self.K2_SetActorRotation` _array_element_2 (`KismetMathLibrary.ComposeRotators` (`KismetMathLibrary.MakeRotator` 0.0 0.0 (`KismetAnimationLibrary.CalculateDirection` (`SplineComponent.FindTangentClosestToWorldLocation` (`self.Spline`) _returnvalue_3 "Local") _returnvalue)) (`KismetMathLibrary.MakeRotator` _returnvalue_roll _returnvalue_pitch)) false))
              (:`Is Not Valid`
                _))))
        (`KismetArrayLibrary.Array_Add` (`self.MovedActors`) _array_element_2)))))

(fn `UserConstructionScript`)