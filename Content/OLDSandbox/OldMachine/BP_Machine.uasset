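; Crafting machine actor that turns fed-in items into a product, using the hardcoded IronBar row of DT_Recipes.
; An overlap switch toggles power and warm-up; three input boxes destroy items tagged with the ingredient ID and count them.
; A timeline drives the crafting countdown and spawns output at an arrow while stock lasts.
; Wrong items jam it until removed, with material lights, text readouts, shaking and Niagara-style effects signalling state.
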(event `SetRecipie`
  (bind _returnvalue (`|GetDataTableRow` "/Game/OLDSandbox/DataTables/DT_Recipes.DT_Recipes" "IronBar")
    (:`then`
      (bind ((`Name_27_AB28625446E603AB6FBE2B8ECFEDBDE4` _name) (`CraftedItem_25_351FCD6B4C6476B88A92EE8DAEE882D9` _crafteditem) (`SpawnQuantity_47_5C5B71A24494D14E50571B8C83EA2550` _spawnquantity) (`CraftingTime_50_AAFE20554C3DCA4E03CCB2821F056DC8` _craftingtime) (`ItemDescription_14_5A64C405440E8BA0F364D98251634FD2` _itemdescription) (`Required_Item1_52_CA7CDC05460573E35637F4A63889800A` _required_item1) (`Item1_ID_51_DA8CC71449CAFB4A7DEA24B4B268838D` _item1_id) (`Item1_Quantity_39_6716F6044F1C0BB4DEC72C94A873280F` _item1_quantity)) (break `/Game/OLDSandbox/DataTables/S_Recipes` _returnvalue))
      (set `self.Name` _name)
      (set `self.Crafted Item` _crafteditem)
      (set `self.Spawn Quantity` _spawnquantity)
      (set `self.Crafting Time` _craftingtime)
      (set `self.Item Description` _itemdescription)
      (bind _output_get (set `self.Item 1 ID` _item1_id))
      (set `self.Item 1 Quantity` _item1_quantity)
      (`KismetSystemLibrary.PrintString` (`KismetTextLibrary.Conv_TextToString` _output_get)))))

(event `self.ReceiveBeginPlay`
  ;[0.08283 1 0] Begin
  (set `self.SocketL` (`KismetMathLibrary.Conv_VectorToTransform` (`SceneComponent.GetSocketLocation` (`self.Machine`) "MachineLeft")))
  (set `self.InitalRotation` (`SceneComponent.K2_GetComponentRotation` (`self.Machine`)))
  (`self.Power` false))

(event `self.On/Off.OnComponentBeginOverlap`
  (params (OverlappedComponent :type "PrimitiveComponent Object Reference") (OtherActor :type "Actor Object Reference") (OtherComp :type "PrimitiveComponent Object Reference") (OtherBodyIndex :type Integer) (bFromSweep :type Boolean) (SweepResult :type "HitResult Structure (by ref)"))
  ;[1 1 1] Power Switch
  (`/Engine/EditorBlueprintResources/StandardMacros.IsValid` (`GameplayStatics.GetPlayerController` 0)
    (:`Is Valid`
      (`KismetSystemLibrary.Delay` 0.25)
      (`SceneComponent.SetVisibility` (`self.E`) true false)
      (set `self.SwitchON` true)
      (`/Engine/EditorBlueprintResources/StandardMacros.FlipFlop`
        (:`A`
          (`self.Power` true))
        (:`B`
          (`self.Power` false))))))

(event `self.On/Off.OnComponentEndOverlap`
  (params (OverlappedComponent :type "PrimitiveComponent Object Reference") (OtherActor :type "Actor Object Reference") (OtherComp :type "PrimitiveComponent Object Reference") (OtherBodyIndex :type Integer))
  (`/Engine/EditorBlueprintResources/StandardMacros.IsValid` (`GameplayStatics.GetPlayerController` 0)
    (:`Is Valid`
      (`SceneComponent.SetVisibility` (`self.E`) false false)
      (set `self.SwitchON` false))))

(event `Power`
  (params (`On/Off` :type Boolean))
  (bind _returnvalue (`KismetTextLibrary.Conv_StringToText` ""))
  (bind _machine (`self.Machine`))
  ;[1 0.003585 0] Power ON/OFF
  (bind _output_get (set `self.On/ Off` `On/Off`))
  (if _output_get
    (`PrimitiveComponent.SetMaterial` (`self.Machine`) 2 "/Game/Material/M_LightBlue.M_LightBlue")
    (`TextRenderComponent.K2_SetText` (`self.AmountText`) (`|FormatText` "Powering ON"))
    (`KismetSystemLibrary.Delay` 0.25)
    (`self.WarmUp`)
    (`self.SetRecipie`)
    (else
      ;;[0.06771 0.001419 0] OFF
      (`TextRenderComponent.K2_SetText` (`self.ItemText`) _returnvalue)
      (`TextRenderComponent.K2_SetText` (`self.AmountText`) _returnvalue)
      (`TextRenderComponent.K2_SetText` (`self.ItemDescription`) _returnvalue)
      (`TextRenderComponent.K2_SetText` (`self.CraftingTime`) _returnvalue)
      (`KismetSystemLibrary.Delay` 0.5)
      (`PrimitiveComponent.SetMaterial` _machine 2 "/Game/Material/M_LightOff.M_LightOff")
      (`KismetSystemLibrary.Delay` 0.4)
      (`PrimitiveComponent.SetMaterial` _machine 3 "/Game/Material/M_LightOff.M_LightOff"))))

(event `WarmUp`
  ;[1 0.1197 0] Warm Up
  (if (`self.On/ Off`)
    (`KismetSystemLibrary.Delay` 0.25)
    (`PrimitiveComponent.SetMaterial` (`self.Machine`) 3 "/Game/Material/M_LightGreen.M_LightGreen")
    (`KismetSystemLibrary.Delay` 0.15)
    (`PrimitiveComponent.SetMaterial` (`self.Machine`) 2 "/Game/Material/M_LightBlue.M_LightBlue")
    (`KismetSystemLibrary.Delay` 0.15)
    (`TextRenderComponent.K2_SetText` (`self.ItemText`) (`KismetTextLibrary.Conv_StringToText` "..."))
    (`KismetSystemLibrary.Delay` 1.0)
    (`self.SpawnItems`)
    (if (not (`self.On/ Off`))
      (`self.Power` false))))

(event `SpawnItems`
  ;[0 0.1127 1] SpawnItems
  (if (`self.On/ Off`)
    (`TextRenderComponent.K2_SetText` (`self.ItemText`) (`self.Name`))
    (`TextRenderComponent.K2_SetText` (`self.ItemDescription`) (`self.Item Description`))
    (`PrimitiveComponent.SetMaterial` (`self.Machine`) 3 "/Game/Material/M_LightGreen.M_LightGreen")
    (`PrimitiveComponent.SetMaterial` (`self.Machine`) 2 "/Game/Material/M_LightBlue.M_LightBlue")
    (`KismetSystemLibrary.Delay` 1.0)
    (if (`self.Is Jammed`) :!label _label
      (bind (_direction _newtrack_0) (`Timeline|Timeline_0` :`NewTime` (`self.Crafting Time`) :!via `Stop` :!label _label_2)
        (:`Update`
          (`TextRenderComponent.K2_SetText` (`self.CraftingTime`) (`KismetTextLibrary.Conv_DoubleToText` (`KismetMathLibrary.Lerp` (`self.Crafting Time`) 0.0 _newtrack_0) "HalfToEven")))
        (:`Finished`
          (`|SpawnActorFromClass` (`self.Crafted Item`) (`KismetMathLibrary.MakeTransform` (`SceneComponent.K2_GetComponentLocation` (`self.Arrow`))) "Undefined" "SelectDefaultAtRuntime" null null)
          (`self.CounterSubtract`)
          (goto _label)))
      (elif (<= (`self.Counter`) 0)
        (`self.isEmpty` true)
        (goto _label_2 :!via `Stop`)
        (else
          (for _ (range 1)
            (if (`self.On/ Off`)
              (goto _label_2 :!via `PlayFromStart`)
              (else
                (goto _label_2 :!via `Stop`)))))))))

(event `Jammed`
  (params (IsJammed :type Boolean))
  (bind _machine (`self.Machine`))
  (bind _machine_2 (`self.Machine`))
  ;[0.3837 0 0] Jammed
  (if (`self.On/ Off`)
    (bind _output_get (set `self.Is Jammed` IsJammed))
    (if _output_get
      (`PrimitiveComponent.SetMaterial` (`self.Machine`) 2 "/Game/Material/M_LightError.M_LightError")
      (`PrimitiveComponent.SetMaterial` (`self.Machine`) 3 "/Game/Material/M_LightError.M_LightError")
      (`TextRenderComponent.K2_SetText` (`self.ItemText`) (`KismetTextLibrary.Conv_StringToText` "JAMMED"))
      (`KismetSystemLibrary.Delay` 0.5)
      (`NiagaraComponent.ReinitializeSystem` (`self.Explosion`))
      (if (`self.Is Jammed`) :!label _label_3
        (if (`self.On/ Off`)
          (`PrimitiveComponent.SetMaterial` _machine 3 "/Game/Material/M_LightError.M_LightError")
          (`PrimitiveComponent.SetMaterial` _machine 2 "/Game/Material/M_LightError.M_LightError")
          (bind (_direction _newtrack_0) (`Timeline|Timeline` :`NewTime` 0.2 :!label _label_4)
            (:`Update`
              (`SceneComponent.K2_AddLocalRotation` (`self.Machine`) (`KismetMathLibrary.MakeRotator` (* (.x _newtrack_0) 0.3) (* (.y _newtrack_0) 0.3)) false false)
              (`KismetSystemLibrary.Delay` 0.2)
              (`NiagaraComponent.ReinitializeSystem` (`self.Sparks`))
              (`PrimitiveComponent.SetMaterial` _machine_2 3 "/Game/Material/M_LightOff.M_LightOff")
              (`PrimitiveComponent.SetMaterial` _machine_2 2 "/Game/Material/M_LightOff.M_LightOff")
              (`KismetSystemLibrary.Delay` 0.2)
              (goto _label_3))))
        (else
          (goto _label_4 :!via `Stop`)))
      (else
        (`SceneComponent.K2_SetWorldRotation` (`self.Machine`) (`self.InitalRotation`) false false)
        (`self.WarmUp`)))))

(event `self.RightBox.OnComponentBeginOverlap`
  (params (OverlappedComponent :type "PrimitiveComponent Object Reference") (OtherActor :type "Actor Object Reference") (OtherComp :type "PrimitiveComponent Object Reference") (OtherBodyIndex :type Integer) (bFromSweep :type Boolean) (SweepResult :type "HitResult Structure (by ref)"))
  (if (`self.On/ Off`)
    (`/Engine/EditorBlueprintResources/StandardMacros.IsValid` OtherActor
      (:`Is Valid`
        (if (`self.ActorHasTag` OtherActor (`KismetStringLibrary.Conv_StringToName` (`KismetTextLibrary.Conv_TextToString` (`self.Item 1 ID`))))
          (if (not (`self.Is Jammed`))
            (`self.K2_DestroyActor` (`|MakeArray` OtherActor))
            (`self.CounterAdd`))
          (else
            (`self.Jammed` true)))))))

(event `self.LeftBox.OnComponentBeginOverlap`
  (params (OverlappedComponent :type "PrimitiveComponent Object Reference") (OtherActor :type "Actor Object Reference") (OtherComp :type "PrimitiveComponent Object Reference") (OtherBodyIndex :type Integer) (bFromSweep :type Boolean) (SweepResult :type "HitResult Structure (by ref)"))
  (if (`self.On/ Off`)
    (`/Engine/EditorBlueprintResources/StandardMacros.IsValid` OtherActor
      (:`Is Valid`
        (if (`self.ActorHasTag` OtherActor (`KismetStringLibrary.Conv_StringToName` (`KismetTextLibrary.Conv_TextToString` (`self.Item 1 ID`))))
          (if (not (`self.Is Jammed`))
            (`self.K2_DestroyActor` (`|MakeArray` OtherActor))
            (`self.CounterAdd`))
          (else
            (`self.Jammed` true)))))))

(event `self.TopBox.OnComponentBeginOverlap`
  (params (OverlappedComponent :type "PrimitiveComponent Object Reference") (OtherActor :type "Actor Object Reference") (OtherComp :type "PrimitiveComponent Object Reference") (OtherBodyIndex :type Integer) (bFromSweep :type Boolean) (SweepResult :type "HitResult Structure (by ref)"))
  (if (`self.On/ Off`)
    (`/Engine/EditorBlueprintResources/StandardMacros.IsValid` OtherActor
      (:`Is Valid`
        (if (`self.ActorHasTag` OtherActor (`KismetStringLibrary.Conv_StringToName` (`KismetTextLibrary.Conv_TextToString` (`self.Item 1 ID`))))
          (if (not (`self.Is Jammed`))
            (`self.K2_DestroyActor` (`|MakeArray` OtherActor))
            (`self.CounterAdd`))
          (else
            (`self.Jammed` true)))))))

(event `self.RightBox.OnComponentEndOverlap`
  (params (OverlappedComponent :type "PrimitiveComponent Object Reference") (OtherActor :type "Actor Object Reference") (OtherComp :type "PrimitiveComponent Object Reference") (OtherBodyIndex :type Integer))
  (`/Engine/EditorBlueprintResources/StandardMacros.IsValid` OtherActor
    (:`Is Valid`
      (if (not (`self.ActorHasTag` OtherActor (`KismetStringLibrary.Conv_StringToName` (`KismetTextLibrary.Conv_TextToString` (`self.Item 1 ID`)))))
        (`self.Jammed` false)))))

(event `self.LeftBox.OnComponentEndOverlap`
  (params (OverlappedComponent :type "PrimitiveComponent Object Reference") (OtherActor :type "Actor Object Reference") (OtherComp :type "PrimitiveComponent Object Reference") (OtherBodyIndex :type Integer))
  (`/Engine/EditorBlueprintResources/StandardMacros.IsValid` OtherActor
    (:`Is Valid`
      (if (not (`self.ActorHasTag` OtherActor (`KismetStringLibrary.Conv_StringToName` (`KismetTextLibrary.Conv_TextToString` (`self.Item 1 ID`)))))
        (`self.Jammed` false)))))

(event `self.TopBox.OnComponentEndOverlap`
  (params (OverlappedComponent :type "PrimitiveComponent Object Reference") (OtherActor :type "Actor Object Reference") (OtherComp :type "PrimitiveComponent Object Reference") (OtherBodyIndex :type Integer))
  (`/Engine/EditorBlueprintResources/StandardMacros.IsValid` OtherActor
    (:`Is Valid`
      (if (not (`self.ActorHasTag` OtherActor (`KismetStringLibrary.Conv_StringToName` (`KismetTextLibrary.Conv_TextToString` (`self.Item 1 ID`)))))
        (`self.Jammed` false)))))

(event `CounterAdd`
  ;[1 1 1] Counter
  (if (`self.On/ Off`)
    (bind _result (`/Engine/EditorBlueprintResources/StandardMacros.IncrementInt` (`self.Counter`))
      (:`  `
        (`TextRenderComponent.K2_SetText` (`self.AmountText`) (`|FormatText` "Amount {x}/{y} " (`KismetTextLibrary.Conv_IntToText` _result) (`self.Counter Max`)))
        (if (> (`self.Counter`) 0)
          (`self.isEmpty` false))))))

(event `CounterSubtract`
  ;[1 1 1] Counter
  (if (`self.On/ Off`)
    (bind _output_get (set `self.Counter` (- (`self.Counter`) 1)))
    (`TextRenderComponent.K2_SetText` (`self.AmountText`) (`|FormatText` "Amount {x}/{y} " (`KismetTextLibrary.Conv_IntToText` _output_get) (`self.Counter Max`)))))

(event `isEmpty`
  (params (Empty :type Boolean))
  (bind _output_get (set `self.IsEmpty?` Empty))
  (if (`self.On/ Off`)
    (if (not (`self.Is Jammed`))
      (if _output_get :!label _label_5
        (if (`self.On/ Off`)
          (`TextRenderComponent.K2_SetText` (`self.ItemText`) (`KismetTextLibrary.Conv_StringToText` "EMPTY"))
          (`PrimitiveComponent.SetMaterial` (`self.Machine`) 3 "/Game/Material/M_LightError.M_LightError")
          (`PrimitiveComponent.SetMaterial` (`self.Machine`) 2 "/Game/Material/M_LightBlue.M_LightBlue")
          (`KismetSystemLibrary.Delay` 0.5)
          (goto _label_5))
        (else
          (`self.SpawnItems`))))))

(fn `UserConstructionScript`)