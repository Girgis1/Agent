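; BoxforBott is a plastic box prop with adjustable color and dirt, plus an impact sound.
; The construction script creates a dynamic instance of the plastic material, sets its Color and Dirt parameters, and applies it to the first four material slots.
; On component hit, a plastic box sound plays at the box's location when the normal impulse magnitude falls within a set range.
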(event `self.Box.OnComponentHit`
  (params (HitComponent :type "PrimitiveComponent Object Reference") (OtherActor :type "Actor Object Reference") (OtherComp :type "PrimitiveComponent Object Reference") (NormalImpulse :type "Vector Structure") (Hit :type "HitResult Structure (by ref)"))
  (if (`KismetMathLibrary.InRange_FloatFloat` (`KismetMathLibrary.VSize` NormalImpulse) 3000.0 90000.0)
    (`GameplayStatics.PlaySoundAtLocation` "/Game/OLDSandbox/Trash_Pack_Vol_4/Sounds/PlasticBox.PlasticBox" (`SceneComponent.K2_GetComponentLocation` (`self.Box`)) (struct) 0.5 1.0 0.0 null null null null)))

(fn `UserConstructionScript`
  (bind _dynomaterial (`self.DynoMaterial`))
  (bind _box (`self.Box`))
  (bind _returnvalue (`PrimitiveComponent.CreateDynamicMaterialInstance` _box 0 "/Game/OLDSandbox/Trash_Pack_Vol_4/Materials/Plastic_models.Plastic_models" "None"))
  (set `self.DynoMaterial` _returnvalue)
  (`MaterialInstanceDynamic.SetVectorParameterValue` _dynomaterial "Color" (`self.Color_`))
  (`MaterialInstanceDynamic.SetScalarParameterValue` _dynomaterial "Dirt" (`self.Dirt`))
  (`PrimitiveComponent.SetMaterial` _box 0 _dynomaterial)
  (`PrimitiveComponent.SetMaterial` _box 1 _dynomaterial)
  (`PrimitiveComponent.SetMaterial` _box 2 _dynomaterial)
  (`PrimitiveComponent.SetMaterial` _box 3 _dynomaterial))