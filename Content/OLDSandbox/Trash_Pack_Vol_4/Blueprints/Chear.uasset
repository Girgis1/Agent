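; Physics prop Blueprint, apparently a plastic chair, that reacts to impacts on its Chear component.
; Hits with impulse magnitude inside a set range play a plastic sound at the component, then wait one second.
; Impulses under a lower threshold then add a Geometry Collection component at the component's relative transform, without removing the original; stronger ones only print debug text.
; An unconnected SpawnActor node is left unused.
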(event `self.Chear.OnComponentHit`
  (params (HitComponent :type "PrimitiveComponent Object Reference") (OtherActor :type "Actor Object Reference") (OtherComp :type "PrimitiveComponent Object Reference") (NormalImpulse :type "Vector Structure") (Hit :type "HitResult Structure (by ref)"))
  (bind _returnvalue (`KismetMathLibrary.VSize` NormalImpulse))
  (if (`KismetMathLibrary.InRange_FloatFloat` _returnvalue 5000.0 90000.0)
    (`GameplayStatics.PlaySoundAtLocation` "/Game/OLDSandbox/Trash_Pack_Vol_4/Sounds/PlasticChe.PlasticChe" (`SceneComponent.K2_GetComponentLocation` (`self.Chear`)) (struct) 1.0 1.0 0.0 null null null null)
    (`KismetSystemLibrary.Delay` 1.0)
    (if (> 10000.0 _returnvalue)
      (`AddComponent|NODE_AddGeometryCollectionComponent-5` :`RelativeTransform` (`SceneComponent.GetRelativeTransform` (`self.Chear`)))
      (`KismetSystemLibrary.PrintString` "Hello")
      (else
        (`KismetSystemLibrary.PrintString` "na")))))

(fn `UserConstructionScript`)