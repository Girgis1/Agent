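; Old_Bank is an old paint can prop with a configurable color and an optional open-lid mesh.
; The construction script swaps in the open mesh when Open is set, then applies a dynamic M_PaintCan material tinted by Color0 to both material slots.
; On a hit, it plays an impact sound at the can's location if the impulse magnitude falls within a set range.
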(event `self.ReceiveHit`
  (params (MyComp :type "PrimitiveComponent Object Reference") (Other :type "Actor Object Reference") (OtherComp :type "PrimitiveComponent Object Reference") (bSelfMoved :type Boolean) (HitLocation :type "Vector Structure") (HitNormal :type "Vector Structure") (NormalImpulse :type "Vector Structure") (Hit :type "HitResult Structure (by ref)"))
  (if (`KismetMathLibrary.InRange_FloatFloat` (`KismetMathLibrary.VSize` NormalImpulse) 2500.0 90000.0 true false)
    (`GameplayStatics.PlaySoundAtLocation` "/Game/OLDSandbox/Trash_Pack_Vol_4/Sounds/Bank_Cue.Bank_Cue" (`SceneComponent.K2_GetComponentLocation` (`self.PaintCan_Old_1`)) (struct) 0.4 1.0 0.0 null null null null)))

(fn `UserConstructionScript`
  (bind _paintcan_old_1 (`self.PaintCan_Old_1`))
  (if (`self.Open`)
    (`StaticMeshComponent.SetStaticMesh` _paintcan_old_1 "/Game/OLDSandbox/Trash_Pack_Vol_4/Meshes/PaintCan_Old_open.PaintCan_Old_open"))
  (bind _returnvalue (`PrimitiveComponent.CreateDynamicMaterialInstance` _paintcan_old_1 0 "/Game/OLDSandbox/Trash_Pack_Vol_4/Materials/M_PaintCan.M_PaintCan" "None"))
  (bind _output_get (set `self.NewVar` _returnvalue))
  (`MaterialInstanceDynamic.SetVectorParameterValue` _output_get "Color" (`self.Color_0`))
  (`PrimitiveComponent.SetMaterial` _paintcan_old_1 0 _output_get)
  (`PrimitiveComponent.SetMaterial` _paintcan_old_1 1 _output_get))