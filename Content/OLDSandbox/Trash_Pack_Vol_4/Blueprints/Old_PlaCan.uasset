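; Old plastic can prop Blueprint from a trash pack, with an optional open variant and a configurable color.
; The construction script swaps in the open mesh when Open is set and applies one color-parameterized dynamic material instance to three material slots.
; On Hit, it plays a plastic impact sound at the can's location when the impulse magnitude falls within a set range.
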(event `self.ReceiveHit`
  (params (MyComp :type "PrimitiveComponent Object Reference") (Other :type "Actor Object Reference") (OtherComp :type "PrimitiveComponent Object Reference") (bSelfMoved :type Boolean) (HitLocation :type "Vector Structure") (HitNormal :type "Vector Structure") (NormalImpulse :type "Vector Structure") (Hit :type "HitResult Structure (by ref)"))
  (if (`KismetMathLibrary.InRange_FloatFloat` (`KismetMathLibrary.VSize` NormalImpulse) 3000.0 90000.0 true false)
    (`GameplayStatics.PlaySoundAtLocation` "/Game/OLDSandbox/Trash_Pack_Vol_4/Sounds/PlasticBox.PlasticBox" (`SceneComponent.K2_GetComponentLocation` (`self.OldCan_1`)) (struct) 0.4 1.0 0.0 null null null null)))

(fn `UserConstructionScript`
  (bind _oldcan_1 (`self.OldCan_1`))
  (bind _dynomat (`self.DynoMat`))
  (if (`self.Open`)
    (`StaticMeshComponent.SetStaticMesh` _oldcan_1 "/Game/OLDSandbox/Trash_Pack_Vol_4/Meshes/PlasticCan_Open.PlasticCan_Open"))
  (bind _returnvalue (`PrimitiveComponent.CreateDynamicMaterialInstance` _oldcan_1 0 "/Game/OLDSandbox/Trash_Pack_Vol_4/Materials/Can_old.Can_old" "None"))
  (set `self.DynoMat` _returnvalue)
  (`MaterialInstanceDynamic.SetVectorParameterValue` _dynomat "Color" (`self.Color_`))
  (`PrimitiveComponent.SetMaterial` _oldcan_1 0 _dynomat)
  (`PrimitiveComponent.SetMaterial` _oldcan_1 1 _dynomat)
  (`PrimitiveComponent.SetMaterial` _oldcan_1 2 _dynomat))