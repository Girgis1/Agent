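; Resource node actor that repeatedly spawns items at its Arrow while switched on.
; Each actor overlap, after a short delay, flip-flops the node on or off, swapping the mesh material and calling Power.
; Power loops through a SpawnTime delay, spawning AssignedActor or, without SetItem, adding a child actor component.
; BeginPlay only sets the material from OnOff, without starting the spawn loop.
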(event `self.ReceiveBeginPlay`
  (if (`self.On/ Off`)
    (`PrimitiveComponent.SetMaterial` (`self.StaticMesh`) 0 "/Game/StarterContent/Materials/M_Basic_Wall.M_Basic_Wall")
    (else
      (`PrimitiveComponent.SetMaterial` (`self.StaticMesh`) 0 "/Game/Resources/Material_OFF.Material_OFF"))))

(event `self.ReceiveTick`
  (params (DeltaSeconds :type "Float (single-precision)")))

(event `Power`
  (params (`On/Off` :type Boolean))
  (bind _output_get (set `self.On/ Off` `On/Off`))
  (if _output_get :!label _label
    (for _ (range 1)
      (if (`self.Set Item`)
        (bind _returnvalue (`GameplayStatics.GetActorOfClass` (`self.Assigned Actor`)))
        (`|SpawnActorFromClass` (`self.Assigned Actor`) (`KismetMathLibrary.MakeTransform` (`SceneComponent.K2_GetComponentLocation` (`self.Arrow`)) (struct) (`self.GetActorRelativeScale3D` _returnvalue)) "Undefined" "SelectDefaultAtRuntime" null null)
        (`KismetSystemLibrary.Delay` (`self.SpawnTime`))
        (goto _label)
        (else
          (`AddComponent|NODE_AddChildActorComponent-2` :`RelativeTransform` (`KismetMathLibrary.Conv_VectorToTransform` (`SceneComponent.RelativeLocation` (`self.Arrow`))))
          (`KismetSystemLibrary.Delay` (`self.SpawnTime`))
          (goto _label))))))

(event `self.ReceiveActorBeginOverlap`
  (params (OtherActor :type "Actor Object Reference"))
  (`KismetSystemLibrary.Delay` 0.25)
  (`/Engine/EditorBlueprintResources/StandardMacros.FlipFlop`
    (:`A`
      (`KismetSystemLibrary.PrintString` "Node: ON" true false (struct :`G` 1.0 :`B` 0.461976 :`A` 1.0))
      (`PrimitiveComponent.SetMaterial` (`self.StaticMesh`) 0 "/Game/StarterContent/Materials/M_Basic_Wall.M_Basic_Wall")
      (`self.Power` true))
    (:`B`
      (`KismetSystemLibrary.PrintString` "Node: OFF" true false (struct :`G` 1.0 :`B` 0.461976 :`A` 1.0))
      (`PrimitiveComponent.SetMaterial` (`self.StaticMesh`) 0 "/Game/Resources/Material_OFF.Material_OFF")
      (`self.Power` false))))

(event `self.Box.OnComponentBeginOverlap`
  (params (OverlappedComponent :type "PrimitiveComponent Object Reference") (OtherActor :type "Actor Object Reference") (OtherComp :type "PrimitiveComponent Object Reference") (OtherBodyIndex :type Integer) (bFromSweep :type Boolean) (SweepResult :type "HitResult Structure (by ref)")))

(fn `UserConstructionScript`)