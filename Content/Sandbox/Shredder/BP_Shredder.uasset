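; BP_Shredder is a sandbox shredder actor that destroys actors entering its kill zone.
; Tick pitches the two shredder components by a fixed step each frame, so spin speed depends on frame rate.
; Overlapping the DestoryZone component destroys any valid other actor; the "Item" tag check has no effect because both branches destroy it.
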(event `self.ReceiveTick`
  (params (DeltaSeconds :type "Float (single-precision)"))
  (`SceneComponent.K2_AddLocalRotation` (`self.Shredder01`) (`KismetMathLibrary.MakeRotator` 0.0 -3.0) false false)
  (`SceneComponent.K2_AddLocalRotation` (`self.Shredder02`) (`KismetMathLibrary.MakeRotator` 0.0 -3.0) false false))

(event `self.DestoryZone.OnComponentBeginOverlap`
  (params (OverlappedComponent :type "PrimitiveComponent Object Reference") (OtherActor :type "Actor Object Reference") (OtherComp :type "PrimitiveComponent Object Reference") (OtherBodyIndex :type Integer) (bFromSweep :type Boolean) (SweepResult :type "HitResult Structure (by ref)"))
  (`/Engine/EditorBlueprintResources/StandardMacros.IsValid` OtherActor
    (:`Is Valid`
      (if (`self.ActorHasTag` OtherActor "Item")
        (`self.K2_DestroyActor` OtherActor)
        (else
          (`self.K2_DestroyActor` OtherActor))))))

(fn `UserConstructionScript`)