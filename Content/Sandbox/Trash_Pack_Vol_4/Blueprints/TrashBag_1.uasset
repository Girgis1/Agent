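; Physics trash bag prop on a skeletal mesh, with configurable color and gloss and randomized size and mass.
; The construction script builds a dynamic material from M_Bags, then randomizes uniform scale and multiplies the current mass scale by a random factor, so both re-roll whenever it runs.
; On hit, impulses within a set strength range play a trash sound at the mesh location and print its mass to screen.
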(event `self.ReceiveHit`
  (params (MyComp :type "PrimitiveComponent Object Reference") (Other :type "Actor Object Reference") (OtherComp :type "PrimitiveComponent Object Reference") (bSelfMoved :type Boolean) (HitLocation :type "Vector Structure") (HitNormal :type "Vector Structure") (NormalImpulse :type "Vector Structure") (Hit :type "HitResult Structure (by ref)"))
  (if (`KismetMathLibrary.InRange_FloatFloat` (`KismetMathLibrary.VSize` NormalImpulse) 5000.0 90000.0)
    (`GameplayStatics.PlaySoundAtLocation` "/Game/Sandbox/Trash_Pack_Vol_4/Sounds/TrashPocket_CUE.TrashPocket_CUE" (`SceneComponent.K2_GetComponentLocation` (`self.SkeletalMeshComponent`)) (struct) 0.6 1.0 0.0 null null null null)
    (`KismetSystemLibrary.PrintString` (`KismetStringLibrary.Conv_DoubleToString` (`PrimitiveComponent.GetMass` (`self.SkeletalMeshComponent`))))))

(fn `UserConstructionScript`
  (bind _skeletalmeshcomponent (`self.SkeletalMeshComponent`))
  (bind _skeletalmeshcomponent_2 (`self.SkeletalMeshComponent`))
  (bind _dynomat (`self.DynoMat`))
  (bind _returnvalue (`PrimitiveComponent.CreateDynamicMaterialInstance` _skeletalmeshcomponent_2 0 "/Game/Sandbox/Trash_Pack_Vol_4/Materials/M_Bags.M_Bags" "None"))
  (set `self.DynoMat` _returnvalue)
  (`MaterialInstanceDynamic.SetVectorParameterValue` _dynomat "Color" (`self.Color_`))
  (`MaterialInstanceDynamic.SetScalarParameterValue` _dynomat "SUB" (`self.Gloss`))
  (`PrimitiveComponent.SetMaterial` _skeletalmeshcomponent_2 0 _dynomat)
  (`SceneComponent.SetRelativeScale3D` (`self.SkeletalMeshComponent`) (`KismetMathLibrary.Conv_DoubleToVector` (`KismetMathLibrary.RandomFloatInRange` 0.75 1.5)))
  (`PrimitiveComponent.SetMassScale` _skeletalmeshcomponent "None" (* (`PrimitiveComponent.GetMassScale` _skeletalmeshcomponent "None") (`KismetMathLibrary.RandomFloatInRange` 1.0 7.0))))